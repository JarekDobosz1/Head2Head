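; AI controller Blueprint that drives Player 2 when the saved game has AI mode on.
; On BeginPlay it caches the game mode and both players, then checks that flag after a short delay.
; A self-restarting timer with randomized intervals feeds Player 2 random horizontal input, slightly biased toward positive values.
; A Jump event exists, but its distance-based trigger is disconnected, so the AI never jumps.
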(event Custom|Jump
  ;[0 0 0] Manual Jump (event tick)
  (Default|JumpEvent (Variables|Default|GetPlayer2) false)
  (Development|PrintString "ai Jump" true true "(R=1.000000,G=1.000000,B=1.000000,A=1.000000)"))

(event Custom|SetInputX
  (if (Variables|Default|GetInitialAiPauseDone)
    (Utilities|Time|ClearandInvalidateTimerbyHandle (Variables|Default|GetMoveTimer))
    (bind _output_get (Variables|Default|SetMoveTimerFrequency (Math|Random|RandomFloatinRange 0.1 0.3)))
    (bind _returnvalue (Utilities|Time|SetTimerbyEvent (delegate Custom|SetInputX) _output_get true))
    (Variables|Default|SetMoveTimer _returnvalue)
    (Variables|/Game/BP_Character.BP_Character_C|SetAction%20Value%20X (Variables|Default|GetPlayer2) (select (Math|Float|InRange(Float) (Math|Random|RandomFloatinRange 0.0 1e+02) 0.0 45.0 true false) (Math|Random|RandomFloatinRange -1.0 0.0) (Math|Random|RandomFloatinRange 0.0 1.0)))))

(event EventBeginPlay
  (Development|PrintString "AI Controller INIT" true true "(R=1.000000,G=0.000000,B=0.923067,A=1.000000)" 5.0)
  (Utilities|FlowControl|Sequence
    (:then_0
      (|Refs))
    (:then_1
      ;[1 1 1] Is game in AI mode?
      (Utilities|FlowControl|Delay 0.1)
      (if (Variables|/Game/BP_SaveGame.BP_SaveGame_C|GetAiMode (Variables|/Game/BP_H2H_GameMode.BP_H2H_GameMode_C|GetSaveGame (Variables|Default|GetGameMode)))
        (Development|PrintString "AI Controller mode on" true true "(R=1.000000,G=0.000000,B=0.923067,A=1.000000)" 5.0)
        (Variables|Default|SetInitialAiPauseDone true)
        (bind _returnvalue (Utilities|Time|SetTimerbyEvent (delegate Custom|SetInputX) (stale Custom|SetInputX _output_get) true))
        (Variables|Default|SetMoveTimer _returnvalue)
        (Variables|/Game/BP_Character.BP_Character_C|SetAction%20Value%20X (Variables|Default|GetPlayer2) (select (Math|Float|InRange(Float) (Math|Random|RandomFloatinRange 0.0 1e+02) 0.0 45.0 true false) (Math|Random|RandomFloatinRange -1.0 0.0) (Math|Random|RandomFloatinRange 0.0 1.0)))))))

(fn ConstructionScript)