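; BP_Camera is a shared camera actor that frames two players, Player1 and Player2.
; Each Tick it moves to the players' midpoint on X and keeps its starting height from BeginPlay.
; Its Y shifts from the start position in proportion to how far player separation differs from a fixed baseline, giving an unclamped distance-based dolly.
; A debug print of a zero vector also runs every frame.
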(event EventBeginPlay
  (Variables|Default|SetInitLocation (Transformation|GetActorLocation)))

(event Collision|EventActorBeginOverlap
  (params (OtherActor :type Actor%20Object%20Reference)))

(event EventTick
  (params (DeltaSeconds :type Float%20%28single-precision%29))
  (bind _player1 (Variables|Default|GetPlayer1))
  (bind _player2 (Variables|Default|GetPlayer2))
  (bind _initlocation (Variables|Default|GetInitLocation))
  (bind _returnvalue (Transformation|GetActorLocation _player1))
  (bind _returnvalue_2 (Transformation|GetActorLocation _player2))
  (bind _returnvalue_3 (Math|Vector|Distance(Vector) _returnvalue _returnvalue_2))
  (bind _returnvalue_4 (- _returnvalue_3 3e+03))
  (bind _returnvalue_5 (* _returnvalue_4 0.55))
  (bind _returnvalue_6 (+ _initlocation (Math|Vector|MakeVector 0.0 _returnvalue_5 0.0)))
  (Transformation|SetActorLocation (Math|Vector|MakeVector (/ (.x (+ _returnvalue _returnvalue_2)) 2.0) (.y _returnvalue_6) (.z _returnvalue_6)) false false)
  (Development|PrintString (Utilities|String|ToString(Vector) "0, 0, 0") true true "(R=0.908823,G=1.000000,B=0.013598,A=1.000000)" 0.0))

(fn ConstructionScript)