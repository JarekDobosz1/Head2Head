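; Character for a two-player head-to-head game, where opponents move along X in mirrored directions chosen by a Player1 class check.
; Each tick, input accumulates a clamped lean that drives movement and body roll, then prints debug values.
; Jumps add an impulse from head orientation and a velocity exponent, gated by a one-second DoOnce reset.
; Helmet and arm overlaps report head-smash or push-down wins to the GameMode.
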(event EventBeginPlay
  (bind _asbp_h2h_game_mode (Utilities|Casting|CastToBP_H2H_GameMode (Game|GetGameMode)))
  (Variables|Default|SetGameModeRef _asbp_h2h_game_mode))

(event EventTick
  (params (DeltaSeconds :type Float%20%28single-precision%29))
  (Utilities|FlowControl|Sequence
    (:then_0
      (|Locomotion))
    (:then_2
      (|Debug))))

(fn ConstructionScript)

(fn IsPlayer1
  (return (== (Utilities|GetClass self) "/Game/BP_Player1.BP_Player1_C")))

(event Custom|JumpEvent
  (params (Pressed :type Boolean))
  (bind _currentvelocity (Variables|Default|GetCurrentVelocity))
  (bind _minimalverticaljump (Variables|Default|GetMinimalVerticalJump))
  (bind _velocityjumpexponent (Variables|Default|GetVelocityJumpExponent))
  (bind _jumpstrength (Variables|Default|GetJumpStrength))
  (bind _headmesh (Variables|Default|GetHeadMesh))
  (bind _returnvalue (Transformation|GetWorldRotation _headmesh))
  (bind _returnvalue_2 (Math|Float|Power _currentvelocity _velocityjumpexponent))
  (bind _returnvalue_3 (Math|Vector|GetUpVector _returnvalue))
  (bind _returnvalue_4 (* _returnvalue_3 _jumpstrength))
  (bind _returnvalue_5 (+ (.z _returnvalue_4) _jumpstrength _returnvalue_2 _minimalverticaljump))
  (bind _returnvalue_6 (Math|Vector|MakeVector (.x _returnvalue_4) (.y _returnvalue_4) _returnvalue_5))
  (Utilities|FlowControl|Sequence
    (:then_0
      (Utilities|FlowControl|DoOnce false :!label _label
        (:Completed
          (Physics|AddImpulse (Variables|Character|GetCharacterMovement) _returnvalue_6 true)
          (Development|PrintString (Utilities|String|Append "Jump Impulse: " (Utilities|String|ToString(Vector) _returnvalue_6)) true true "(R=1.000000,G=0.929495,B=0.000000,A=1.000000)")
          (Development|PrintString (Utilities|String|Append "JumpSqrt:  " (Utilities|String|ToString(Float) _returnvalue_2)) true true "(R=1.000000,G=0.929495,B=0.000000,A=1.000000)"))))
    (:then_1
      (Utilities|FlowControl|Delay 1.0)
      (goto _label Reset))))

(event OnComponentBeginOverlap(ArmsCollision)
  (params (OverlappedComponent :type Primitive%20Component%20Object%20Reference) (OtherActor :type Actor%20Object%20Reference) (OtherComp :type Primitive%20Component%20Object%20Reference) (OtherBodyIndex :type Integer) (bFromSweep :type Boolean) (SweepResult :type Hit%20Result%20Structure%20%28by%20ref%29))
  (if (!= OtherActor self)
    (if (Utilities|Enum|Equal(Enum) (Collision|GetCollisionObjectType OtherComp) "ECC_GameTraceChannel2")
      (Utilities|FlowControl|Sequence
        (:then_0
          (bind _asbp_character (Utilities|Casting|CastToBP_Character OtherActor))
          (Default|PushDownIntotheMud (Variables|Default|GetGameModeRef) self _asbp_character))))))

(event OnComponentBeginOverlap(HelmetCollision)
  (params (OverlappedComponent :type Primitive%20Component%20Object%20Reference) (OtherActor :type Actor%20Object%20Reference) (OtherComp :type Primitive%20Component%20Object%20Reference) (OtherBodyIndex :type Integer) (bFromSweep :type Boolean) (SweepResult :type Hit%20Result%20Structure%20%28by%20ref%29))
  (if (!= OtherActor self)
    (if (Utilities|Enum|Equal(Enum) (Collision|GetCollisionObjectType OtherComp) "ECC_GameTraceChannel1")
      (Utilities|FlowControl|Sequence
        (:then_0
          (bind _asbp_character (Utilities|Casting|CastToBP_Character OtherActor))
          (Default|HeadFaceSmash (Variables|Default|GetGameModeRef) self _asbp_character))))))