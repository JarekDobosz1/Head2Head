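; Game mode for a two-player head-to-head game that resolves helmet and head collisions into a winner and loser, and slows time when the players get close.
; Face smash and push-into-mud events use gates and DoOnce so the first blocks the other.
; Each turns the struck meshes red and calls LaunchAndRagdoll, which launches the loser as a ragdoll with force scaled from winner speed and clamped.
; Reset reloads the game level.
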(event Custom|Reset
  (Game|OpenLevel(byName) "L_game"))

(event EventBeginPlay
  ;[0.7224 0.2493 1] Refs
  (|Refs))

(event EventTick
  (params (DeltaSeconds :type Float%20%28single-precision%29))
  (bind _player1 (Variables|Default|GetPlayer1))
  (Utilities|IsValid _player1
    (:Is%20Valid
      (if (< (Math|Vector|Distance(Vector) (Transformation|GetActorLocation _player1) (Transformation|GetActorLocation (Variables|Default|GetPlayer2))) (Variables|Default|GetSlowMoDistance))
        (Utilities|Time|SetGlobalTimeDilation 0.2)))))

(fn ConstructionScript)

(fn LaunchandRagdoll
  (params (ImpulseType :type Float%20%28double-precision%29) (WinnerSpeedAfter :type Float%20%28single-precision%29))
  (bind _returnvalue (Math|Random|RandomFloatinRange 0.05 0.5))
  (bind _winningplayer (Variables|Default|GetWinningPlayer))
  (bind _winningplayer_2 (Variables|Default|GetWinningPlayer))
  (bind _losingplayer (Variables|Default|GetLosingPlayer))
  (bind _losingplayer_2 (Variables|Default|GetLosingPlayer))
  (bind _helmetcollision (Variables|/Game/BP_Character.BP_Character_C|GetHelmetCollision _losingplayer))
  (bind _charactermovement (Variables|/Script/Engine.Character|GetCharacterMovement _losingplayer))
  (bind _mesh (Variables|/Script/Engine.Character|GetMesh _losingplayer_2))
  (bind _charactermovement_2 (Variables|/Script/Engine.Character|GetCharacterMovement _winningplayer_2))
  (bind _helmetcollision_2 (Variables|/Game/BP_Character.BP_Character_C|GetHelmetCollision _winningplayer))
  (bind _returnvalue_2 (Transformation|GetWorldLocation _helmetcollision_2))
  (bind _returnvalue_3 (Transformation|GetWorldLocation _helmetcollision))
  (bind _returnvalue_4 (- _returnvalue_3 _returnvalue_2))
  (bind _returnvalue_5 (Math|Vector|Normalize (Math|Vector|MakeVector (.x _returnvalue_4) _returnvalue (.z _returnvalue_4))))
  (bind _returnvalue_6 (* _returnvalue_5 ImpulseType))
  ;[1 1 1] Clear current velocity
  (Variables|/Script/Engine.MovementComponent|SetVelocity _charactermovement_2 (* (Variables|/Script/Engine.MovementComponent|GetVelocity _charactermovement_2) WinnerSpeedAfter))
  (Variables|/Script/Engine.MovementComponent|SetVelocity _charactermovement "0, 0, 0")
  ;[1 1 1] Actual Launch of the capsule
  (Physics|AddImpulse _charactermovement _returnvalue_6 true)
  (Utilities|FlowControl|Sequence
    (:then_0
      ;[1 1 1] Launch of the ragdoll
      (Physics|SetPhysicsLinearVelocity _mesh (* _returnvalue_6 1e+01) false "None")
      (Physics|SetSimulatePhysics _mesh true))
    (:then_1
      ;[1 1 1] Debug
      (Rendering|Debug|DrawDebugLine _returnvalue_3 _returnvalue_6 "(R=1.000000,G=0.076467,B=0.000000,A=1.000000)" 5.0 1.0)
      (Development|PrintString (Utilities|String|Append "Launch force: " (Utilities|String|ToString(Float) ImpulseType)) true true "(R=1.000000,G=0.439928,B=0.876865,A=1.000000)" 4.0))))

(fn SetConflictRefs
  (params (WinningPlayer :type BP%20Character%20Object%20Reference))
  (bind _output_get (Variables|Default|SetWinningPlayer WinningPlayer))
  (Variables|Default|SetWinningPlayerVelocity (Variables|/Game/BP_Character.BP_Character_C|GetCurrentVelocity _output_get))
  (Variables|Default|SetLosingPlayer (select (== (Variables|Default|GetWinningPlayer) (Variables|Default|GetPlayer1)) (Variables|Default|GetPlayer2) (Variables|Default|GetPlayer1))))

(event Custom|PushDownIntoTheMud
  (params (WinningPlayer :type BP%20Character%20Object%20Reference) (LosingPlayer :type BP%20Character%20Object%20Reference))
  (bind _helmetmesh (Variables|/Game/BP_Character.BP_Character_C|GetHelmetMesh LosingPlayer))
  (CallFunction|SetConflictRefs WinningPlayer)
  ;[1 1 1] Disable every other conflict event
  (Utilities|FlowControl|Sequence
    (:then_0
      (Utilities|FlowControl|Gate false) ; enters at Close
    )
    (:then_1
      (Utilities|FlowControl|Gate false
        (:Exit
          (Utilities|FlowControl|DoOnce false
            (:Completed
              ;[1 1 1] RedMaterials
              (Utilities|FlowControl|Sequence
                (:then_0
                  (Rendering|Material|SetMaterial _helmetmesh 0 "/Game/Materials/MI_TestMaterial_Red.MI_TestMaterial_Red"))
                (:then_1
                  (Rendering|Material|SetMaterial _helmetmesh 0 "/Game/Materials/MI_TestMaterial_Red.MI_TestMaterial_Red"))
                (:then_2
                  (Utilities|FlowControl|Sequence
                    (:then_0
                      (CallFunction|LaunchandRagdoll (Math|Float|Clamp(Float) (* (Variables|Default|GetWinningPlayerVelocity) (Variables|Default|GetPushIntoMudLaunchForce)) 6.5e+02 2e+03) 1.0))
                    (:then_1
                      (Development|PrintString "Gamemode !PUSH INTO THE MUD!" true true "(R=1.000000,G=0.012648,B=0.000000,A=1.000000)" 3.0))))))))))))

(event Custom|HeadFaceSmash
  (params (WinningPlayer :type BP%20Character%20Object%20Reference) (LosingPlayer :type BP%20Character%20Object%20Reference))
  (CallFunction|SetConflictRefs WinningPlayer)
  ;[1 1 1] Disable every other conflict event
  (Utilities|FlowControl|Sequence
    (:then_0
      (Utilities|FlowControl|Gate false) ; enters at Close
    )
    (:then_1
      (Utilities|FlowControl|Gate false
        (:Exit
          (Utilities|FlowControl|DoOnce false
            (:Completed
              ;[1 1 1] RedMaterials
              (Utilities|FlowControl|Sequence
                (:then_0
                  (Rendering|Material|SetMaterial (Variables|/Game/BP_Character.BP_Character_C|GetHelmetMesh WinningPlayer) 0 "/Game/Materials/MI_TestMaterial_Red.MI_TestMaterial_Red"))
                (:then_1
                  (Rendering|Material|SetMaterial (Variables|/Game/BP_Character.BP_Character_C|GetHeadMesh LosingPlayer) 0 "/Game/Materials/MI_TestMaterial_Red.MI_TestMaterial_Red"))
                (:then_2
                  (Utilities|FlowControl|Sequence
                    (:then_0
                      (CallFunction|LaunchandRagdoll (Math|Float|Clamp(Float) (* (Variables|Default|GetWinningPlayerVelocity) (Variables|Default|GetFaceSmashLaunchForce)) 6.5e+02 2e+03) 0.1))
                    (:then_1
                      (Development|PrintString "Gamemode !FACE SMASH!" true true "(R=1.000000,G=0.012648,B=0.000000,A=1.000000)" 3.0))))))))))))